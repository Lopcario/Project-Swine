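; Base enemy for a first-person game, drawn as a Doom-style directional flipbook sprite that yaws to face the camera.
; Each tick it computes the player's angle to its facing, picks front, side or back idle, move or attack animations, then runs timed melee damage.
; Pawn sensing triggers chasing or attacking by range.
; Lethal damage activates an effect, disables collision, plays death animations and destroys the actor after a delay.
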(event OnSeePawn(PawnSensing)
  (params (Pawn :type Pawn%20Object%20Reference))
  (bind _asbp_first_person_character (Utilities|Casting|CastToBP_FirstPersonCharacter Pawn))
  (Variables|Default|SetPlayerController _asbp_first_person_character)
  (bind _output_get (Variables|Attacking|SetDistanceFromPlayer (Math|Vector|Distance(Vector) (Transformation|GetActorLocation _asbp_first_person_character) (Transformation|GetActorLocation))))
  (Development|PrintString (Utilities|String|ToString(Float) _output_get))
  (if (<= (Variables|Attacking|GetDistanceFromPlayer) (Variables|Attacking|GetMeleeRange))
    (bind _output_get_2 (Variables|Attacking|SetIsAttackingPlayer true))
    (Development|PrintString (Utilities|String|ToString(Boolean) _output_get_2))
    (else
      (Variables|Attacking|SetIsAttackingPlayer false)
      (Variables|Default|SetCanSeePlayer true)
      (AI|AIMoveTo self "0, 0, 0" (Variables|Default|GetPlayerController) 5.0 false))))

(event EventBeginPlay
  (Components|Activation|Deactivate (Variables|Default|GetP_Explosion))
  (Variables|/Script/Engine.CharacterMovementComponent|SetMaxWalkSpeed (Variables|Character|GetCharacterMovement) (Variables|Default|GetWalk%20Speed)))

(event Collision|EventActorBeginOverlap
  (params (OtherActor :type Actor%20Object%20Reference)))

(event EventTick
  (params (DeltaSeconds :type Float%20%28single-precision%29))
  (Utilities|FlowControl|Sequence
    (:then_1
      (Utilities|SpriteFacePlayer
        (:out
          (Utilities|GetEnemyAngle
            (:out
              (Utilities|CalculateFlipbook
                (:out
                  (Utilities|MeleeAttack))))))))))

(event Game|Damage|EventAnyDamage
  (params (Damage :type Float%20%28single-precision%29) (DamageType :type Damage%20Type%20Object%20Reference) (InstigatedBy :type Controller%20Object%20Reference) (DamageCauser :type Actor%20Object%20Reference))
  (Variables|TakingDamage|SetHP (- (Variables|TakingDamage|GetHP) Damage))
  (if (<= (Variables|TakingDamage|GetHP) 0.0)
    (Components|Activation|Activate (Variables|Default|GetP_Explosion) false)
    (Variables|TakingDamage|SetIsAlive false)
    (Collision|SetCollisionEnabled (Variables|Collision|GetCapsuleComponent) "NoCollision")
    (Utilities|FlowControl|DoOnce false
      (:Completed
        (Components|Activation|Deactivate (Variables|Character|GetCharacterMovement))
        (Components|Activation|Deactivate (Variables|Default|GetPawnSensing))
        (Utilities|FlowControl|Delay 5.0)
        (Actor|DestroyActor)))))

(fn ConstructionScript)