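; Enemy projectile with a flipbook sprite that damages the player on overlap.
; On spawn it briefly hides the sprite, then a self-repeating delay loop keeps yawing the actor toward the player.
; Overlaps damage Player-tagged actors without destroying the projectile, ignore other projectiles, zero max speed on anything else, and destroy it unless that is an enemy.
; Radius explosion logic is present but unconnected, and the other functions are empty stubs.
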(event OnComponentBeginOverlap(HitRadius)
  (params (OverlappedComponent :type Primitive%20Component%20Object%20Reference) (OtherActor :type Actor%20Object%20Reference) (OtherComp :type Primitive%20Component%20Object%20Reference) (OtherBodyIndex :type Integer) (bFromSweep :type Boolean) (SweepResult :type Hit%20Result%20Structure%20%28by%20ref%29))
  (bind _projectilemovement (Variables|Default|GetProjectileMovement))
  (Variables|Default|SetOther%20Actor OtherActor)
  (if (Actor|ActorHasTag OtherActor "Player")
    (Development|PrintString (Utilities|GetDisplayName (Variables|Default|GetOther%20Actor)))
    (Game|Damage|ApplyDamage (Variables|Default|GetOther%20Actor) 1e+01 0 0)
    (elif (not (Actor|ActorHasTag OtherActor "Projectile"))
      (Variables|/Script/Engine.ProjectileMovementComponent|SetMaxSpeed _projectilemovement 0.0)
      (if (not (Actor|ActorHasTag OtherActor "Enemy"))
        (Variables|/Script/Engine.MovementComponent|SetVelocity _projectilemovement "0, 0, 0")
        (Actor|DestroyActor)))))

(event Custom|Face%20Playerr
  ;[1 1 1] Forces sprite to face player
  (Transformation|SetActorRotation (Math|Rotator|MakeRotator 0.0 0.0 (.yaw (Math|Interpolation|RInterpTo (Transformation|GetActorRotation) (Math|Rotator|FindLookatRotation (Transformation|GetActorLocation) (Transformation|GetActorLocation (Variables|Default|GetCharRef))) (Utilities|Time|GetWorldDeltaSeconds) 2e+01))))
  (Utilities|FlowControl|Delay 0.001)
  (CallFunction|FacePlayerr))

(event EventBeginPlay
  ;[1 1 1] Forces sprite to face player
  (Rendering|SetVisibility (Variables|Default|GetRocketIdleFlipBook) false true)
  (bind _asbp_first_person_character (Utilities|Casting|CastToBP_FirstPersonCharacter (Game|GetPlayerCharacter 0)))
  (Variables|Default|SetCharRef _asbp_first_person_character)
  (CallFunction|FacePlayerr)
  (Utilities|FlowControl|Delay 0.065)
  (Rendering|SetVisibility (Variables|Default|GetRocketIdleFlipBook) true true))

(fn ConstructionScript)

(fn FacePlayer)