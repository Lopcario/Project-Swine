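; Flying ranged enemy drawn as a Doom-style directional flipbook sprite that chases and shoots the first-person player.
; PawnSensing sets the chase or attack state by distance; Tick aims, billboards the sprite and fires projectiles on a cooldown.
; Dot products of enemy facing and player direction select front, side or back flipbooks per state.
; Damage triggers alternating-direction dodge impulses, or explosion, death animation and delayed destruction; MeleeAttack is never called.
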(event OnSeePawn(PawnSensing)
  (params (Pawn :type Pawn%20Object%20Reference))
  (bind _asbp_first_person_character (Utilities|Casting|CastToBP_FirstPersonCharacter Pawn))
  (Variables|Default|SetPlayerController _asbp_first_person_character)
  (Variables|Default|SetPlayerLocal (Transformation|GetActorLocation _asbp_first_person_character))
  (Variables|Attacking|SetDistanceFromPlayer (Math|Vector|Distance(Vector) (Transformation|GetActorLocation _asbp_first_person_character) (Transformation|GetActorLocation)))
  (if (<= (Variables|Attacking|GetDistanceFromPlayer) (Variables|Attacking|GetShootRange))
    (Variables|Attacking|SetIsAttackingPlayer true)
    (else
      (Variables|Attacking|SetIsAttackingPlayer false)
      (Variables|Default|SetCanSeePlayer true)
      (Variables|/Script/Engine.CharacterMovementComponent|SetMaxWalkSpeed (Variables|Character|GetCharacterMovement) 5e+02)
      (AI|AIMoveTo self "0, 0, 0" (Variables|Default|GetPlayerController) 5.0 false))))

(event Custom|Dodge
  (bind _charactermovement (Variables|Character|GetCharacterMovement))
  (bind _dodgearrow (Variables|Default|GetDodgeArrow))
  ;[1 1 1] Dodge
  (Variables|/Script/Engine.MovementComponent|SetVelocity _charactermovement (+ (Variables|/Script/Engine.MovementComponent|GetVelocity _charactermovement) (* (Math|Vector|GetForwardVector (Variables|Default|GetDodgeArrow)) (Variables|Default|GetDodgePower))))
  (Development|PrintString "Impluse Added")
  (Transformation|SetWorldRotation _dodgearrow (Math|Rotator|MakeRotator 0.0 0.0 (+ (.yaw (Transformation|GetWorldRotation _dodgearrow)) 1.8e+02)) false false)
  (Utilities|FlowControl|Delay 0.1))

(event EventBeginPlay
  (Components|Activation|Deactivate (Variables|Default|GetP_Explosion))
  (Variables|/Script/Engine.CharacterMovementComponent|SetMaxWalkSpeed (Variables|Character|GetCharacterMovement) (Variables|Default|GetWalk%20Speed)))

(event Collision|EventActorBeginOverlap
  (params (OtherActor :type Actor%20Object%20Reference)))

(event EventTick
  (params (DeltaSeconds :type Float%20%28single-precision%29))
  (Utilities|FlowControl|Sequence
    (:then_1
      (Utilities|AimatPlayer
        (:Exit
          (Utilities|SpriteFacePlayer
            (:out
              (Utilities|GetEnemyAngle
                (:out
                  (Utilities|CalculateFlipbook
                    (:out
                      (Utilities|RangedAttack))))))))))))

(event Game|Damage|EventAnyDamage
  (params (Damage :type Float%20%28single-precision%29) (DamageType :type Damage%20Type%20Object%20Reference) (InstigatedBy :type Controller%20Object%20Reference) (DamageCauser :type Actor%20Object%20Reference))
  (Variables|TakingDamage|SetHP (- (Variables|TakingDamage|GetHP) Damage))
  (if (<= (Variables|TakingDamage|GetHP) 0.0)
    (Components|Activation|Activate (Variables|Default|GetP_Explosion) false)
    (Variables|TakingDamage|SetIsAlive false)
    (Collision|SetCollisionEnabled (Variables|Collision|GetCapsuleComponent) "NoCollision")
    (Utilities|FlowControl|DoOnce false
      (:Completed
        (Components|Activation|Deactivate (Variables|Character|GetCharacterMovement))
        (Components|Activation|Deactivate (Variables|Default|GetPawnSensing))
        (Utilities|FlowControl|Delay 5.0)
        (Actor|DestroyActor)))
    (else
      (CallFunction|Dodge)
      (Development|PrintString "Hello"))))

(fn ConstructionScript)