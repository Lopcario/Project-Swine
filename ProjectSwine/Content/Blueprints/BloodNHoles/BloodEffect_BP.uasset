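; BloodEffect_BP is a short-lived blood splatter actor that shows a random sprite.
; On BeginPlay it picks a random sprite from its sprite array for the Blood component, then destroys itself after a one-second delay.
; Each Tick it billboards the sprite by yawing it toward the player camera, keeping pitch and roll at zero.
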(event EventBeginPlay
  (Rendering|Components|Sprite|SetSprite (Variables|Default|GetBlood) (.OutItem (Utilities|Array|Random (Variables|Default|GetBlood%20Srites))))
  (Utilities|FlowControl|Delay 1.0)
  (Actor|DestroyActor))

(event Collision|EventActorBeginOverlap
  (params (OtherActor :type Actor%20Object%20Reference)))

(event EventTick
  (params (DeltaSeconds :type Float%20%28single-precision%29))
  (Transformation|SetWorldRotation (Variables|Default|GetBlood) (Math|Rotator|MakeRotator 0.0 0.0 (- (.yaw (Math|Rotator|FindLookatRotation (Transformation|GetWorldLocation (Variables|Default|GetBlood)) (Camera|GetCameraLocation (Game|GetPlayerCameraManager 0)))) 9e+01)) false false))

(fn ConstructionScript)