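; BulletHole_BP1 is a short-lived bullet hole decal actor built from a sprite component.
; On BeginPlay it assigns a random sprite from HoleSprites and destroys itself after a few seconds.
; Each tick it billboards the sprite around the vertical axis, yawing it to face the player camera while keeping pitch and roll at zero.
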(event EventBeginPlay
  (Rendering|Components|Sprite|SetSprite (Variables|Default|GetHole) (.OutItem (Utilities|Array|Random (Variables|Default|GetHole%20Sprites))))
  (Utilities|FlowControl|Delay 5.0)
  (Actor|DestroyActor))

(event Collision|EventActorBeginOverlap
  (params (OtherActor :type Actor%20Object%20Reference)))

(event EventTick
  (params (DeltaSeconds :type Float%20%28single-precision%29))
  (Transformation|SetWorldRotation (Variables|Default|GetHole) (Math|Rotator|MakeRotator 0.0 0.0 (- (.yaw (Math|Rotator|FindLookatRotation (Transformation|GetWorldLocation (Variables|Default|GetHole)) (Camera|GetCameraLocation (Game|GetPlayerCameraManager 0)))) 9e+01)) false false))

(fn ConstructionScript)