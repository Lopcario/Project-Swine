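; Machine gun weapon Blueprint with flipbook animation that fires when ShootWeapon is called.
; A DoOnce gates each shot and resets after the fire flipbook's length, so the animation sets the fire rate.
; Each shot calls FireWeapon, plays a random sound, activates smoke and toggles the muzzle flash on BP_FirstPersonCharacter, found through GetActorOfClass.
; Smoke deactivates after a further delay; StopShooting is empty and a PointLight flash is left unconnected.
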(event Custom|Reset%20Weapon
  (bind _weaponflipbook (Variables|Default|GetWeaponflipbook))
  (Utilities|FlowControl|DoOnce false) ; enters at Reset
)

(event EventBeginPlay
  (Components|Activation|Deactivate (Variables|Default|GetP_Smoke1))
  (|CallParentFunction))

(event Collision|EventActorBeginOverlap
  (params (OtherActor :type Actor%20Object%20Reference))
  (|CallParentFunction OtherActor) ; This node is disabled and will not be called.\nDrag off pins to build functionality.
)

(event EventTick
  (params (DeltaSeconds :type Float%20%28single-precision%29))
  (|CallParentFunction DeltaSeconds))

(event EventShootWeapon
  (bind _weaponflipbook (Variables|Default|GetWeaponflipbook))
  (Utilities|FlowControl|DoOnce false
    (:Completed
      (CallFunction|FireWeapon)
      (Sprite|SetFlipbook _weaponflipbook "/Game/Sprites/DevSpritesReplaceLater/RetroFPSAssets/Weapons/MiniGun/SubmachinegunFire.SubmachinegunFire")
      (bind _returnvalue (Actor|GetActorOfClass "/Game/FirstPerson/Blueprints/BP_FirstPersonCharacter.BP_FirstPersonCharacter_C"))
      (Default|MuzzleFlashon _returnvalue)
      (Audio|PlaySound2D (.OutItem (Utilities|Array|Random (Variables|Default|GetSound))) 0.6 1.0 0.0 0 0)
      (Components|Activation|Activate (Variables|Default|GetP_Smoke1) false)
      (Utilities|FlowControl|Delay (Class|PaperFlipbookComponent|GetFlipbookLength _weaponflipbook))
      (Default|MuzzleFlashOff _returnvalue)
      (Sprite|SetFlipbook (Variables|Default|GetWeaponflipbook) "/Game/Sprites/DevSpritesReplaceLater/RetroFPSAssets/Weapons/MiniGun/SubmachinegunIdle.SubmachinegunIdle")
      (CallFunction|ResetWeapon)
      (Utilities|FlowControl|Delay 1.0)
      (Components|Activation|Deactivate (Variables|Default|GetP_Smoke1)))))

(event EventStopShooting)

(fn ConstructionScript
  (|CallParentFunction))