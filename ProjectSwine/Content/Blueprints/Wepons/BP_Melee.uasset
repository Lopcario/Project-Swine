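; BP_Melee is a melee weapon Blueprint that extends a parent weapon class and animates with Paper2D flipbooks.
; ShootWeapon passes a DoOnce gate, calls FireWeapon, switches to the attack flipbook, plays a sound and activates spark particles.
; After a delay matching the flipbook's length, it restores the idle flipbook, reopens the gate through ResetWeapon and shortly afterward deactivates the sparks.
; StopShooting is empty.
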(event Custom|Reset%20Weapon
  (bind _weaponflipbook (Variables|Default|GetWeaponflipbook))
  (Utilities|FlowControl|DoOnce false) ; enters at Reset
)

(event EventBeginPlay
  (Components|Activation|Deactivate (Variables|Default|GetP_Sparks))
  (|CallParentFunction))

(event Collision|EventActorBeginOverlap
  (params (OtherActor :type Actor%20Object%20Reference))
  (|CallParentFunction OtherActor) ; This node is disabled and will not be called.\nDrag off pins to build functionality.
)

(event EventTick
  (params (DeltaSeconds :type Float%20%28single-precision%29))
  (|CallParentFunction DeltaSeconds) ; This node is disabled and will not be called.\nDrag off pins to build functionality.
)

(event EventShootWeapon
  (bind _weaponflipbook (Variables|Default|GetWeaponflipbook))
  (Utilities|FlowControl|DoOnce false
    (:Completed
      (CallFunction|FireWeapon)
      (Sprite|SetFlipbook _weaponflipbook "/Game/Sprites/DevSpritesReplaceLater/RetroFPSAssets/Weapons/Chainsaw/MeleeAttack.MeleeAttack")
      (Audio|PlaySound2D "/Game/Sprites/DevSpritesReplaceLater/RetroFPSAssets/Weapons/Chainsaw/dssawful.dssawful" 0.6 1.0 0.0 0 0)
      (Components|Activation|Activate (Variables|Default|GetP_Sparks) false)
      (Utilities|FlowControl|Delay (Class|PaperFlipbookComponent|GetFlipbookLength _weaponflipbook))
      (Sprite|SetFlipbook (Variables|Default|GetWeaponflipbook) "/Game/Sprites/DevSpritesReplaceLater/RetroFPSAssets/Weapons/Chainsaw/MeleeIDLE.MeleeIDLE")
      (CallFunction|ResetWeapon)
      (Utilities|FlowControl|Delay 0.1)
      (Components|Activation|Deactivate (Variables|Default|GetP_Sparks)))))

(event EventStopShooting)

(fn ConstructionScript
  (|CallParentFunction))