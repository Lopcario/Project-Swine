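; BP_Shotgun is a shotgun weapon that fires single shots with flipbook animation.
; ShootWeapon passes through a DoOnce gate, calls FireWeapon and swaps Weaponflipbook to the fire animation.
; After that flipbook's length it returns to idle, then a short delay later ResetWeapon reopens the gate, so the animation paces the fire rate.
; StopShooting is empty.
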(event Custom|Reset%20Weapon
  (bind _weaponflipbook (Variables|Default|GetWeaponflipbook))
  (Utilities|FlowControl|DoOnce false) ; enters at Reset
)

(event EventBeginPlay
  (|CallParentFunction) ; This node is disabled and will not be called.\nDrag off pins to build functionality.
)

(event Collision|EventActorBeginOverlap
  (params (OtherActor :type Actor%20Object%20Reference))
  (|CallParentFunction OtherActor) ; This node is disabled and will not be called.\nDrag off pins to build functionality.
)

(event EventTick
  (params (DeltaSeconds :type Float%20%28single-precision%29))
  (|CallParentFunction DeltaSeconds) ; This node is disabled and will not be called.\nDrag off pins to build functionality.
)

(event EventShootWeapon
  (bind _weaponflipbook (Variables|Default|GetWeaponflipbook))
  (Utilities|FlowControl|DoOnce false
    (:Completed
      (CallFunction|FireWeapon)
      (Sprite|SetFlipbook _weaponflipbook "/Game/Sprites/DevSprites(ReplaceLater)/RetroFPSAssets/Weapons/Shotgun/shotgunFire.shotgunFire")
      (Utilities|FlowControl|Delay (Class|PaperFlipbookComponent|GetFlipbookLength _weaponflipbook))
      (Sprite|SetFlipbook (Variables|Default|GetWeaponflipbook) "/Game/Sprites/DevSprites(ReplaceLater)/RetroFPSAssets/Weapons/Shotgun/shotgunIdle.shotgunIdle")
      (Utilities|FlowControl|Delay 0.1)
      (CallFunction|ResetWeapon))))

(event EventStopShooting)

(fn ConstructionScript
  (|CallParentFunction))