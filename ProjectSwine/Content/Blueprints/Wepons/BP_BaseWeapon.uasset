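; Base weapon Blueprint that handles hitscan firing for pistol, shotgun and machine gun.
; FireWeapon branches on the first-person character's FireMode; mode 4 only prints a debug string.
; Debug-drawn line traces apply randomized damage, with shotgun and machine gun looping randomly spread traces while they hit.
; Ammo deduction on the character, plus its ShotgunJump and MachineGunGlide calls, happens only along successful-hit paths.
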(event Custom|ShootWeapon)

(event Custom|StopShooting)

(event EventBeginPlay
  (bind _returnvalue (Actor|GetActorOfClass "/Game/FirstPerson/Blueprints/BP_FirstPersonCharacter.BP_FirstPersonCharacter_C")))

(event Collision|EventActorBeginOverlap
  (params (OtherActor :type Actor%20Object%20Reference)))

(event EventTick
  (params (DeltaSeconds :type Float%20%28single-precision%29)))

(fn ConstructionScript)

(fn FireWeapon
  (bind _linetrace (Variables|Default|Getlinetrace))
  (bind _minspreadmachinegun (Variables|MachineGun|GetMinSpreadMachineGun))
  (bind _maxspreadmachinegun (Variables|MachineGun|GetMaxSpreadMachineGun))
  (bind _linetrace_2 (Variables|Default|Getlinetrace))
  (bind _minspreadshotgun (Variables|Shotgun|GetMinSpreadShotgun))
  (bind _maxspreadshotgun (Variables|Shotgun|GetMaxSpreadShotgun))
  (bind _linetrace_3 (Variables|Default|Getlinetrace))
  (bind _returnvalue (Math|Vector|GetForwardVector _linetrace))
  (bind _returnvalue_2 (Transformation|GetWorldLocation _linetrace_3))
  (bind _returnvalue_3 (Transformation|GetWorldLocation _linetrace_2))
  (bind _returnvalue_4 (Transformation|GetWorldLocation _linetrace))
  (bind _returnvalue_5 (Math|Vector|GetForwardVector _linetrace_2))
  (bind _returnvalue_6 (* _returnvalue_5 7.5e+03))
  (bind _returnvalue_7 (* _returnvalue 7.5e+03))
  (bind _returnvalue_8 (+ _returnvalue_4 _returnvalue_7))
  (bind _returnvalue_9 (+ _returnvalue_3 _returnvalue_6))
  (bind (_x _y _z) (Math|Vector|BreakVector _returnvalue_9))
  (bind (_x_2 _y_2 _z_2) (Math|Vector|BreakVector _returnvalue_8))
  (bind _returnvalue_10 (Actor|GetActorOfClass "/Game/FirstPerson/Blueprints/BP_FirstPersonCharacter.BP_FirstPersonCharacter_C"))
  ;[0.4672 1 0.8246] Changes which type of linetrace to fire based on weapon equiped
  (if (== (Variables|/Game/FirstPerson/Blueprints/BP_FirstPersonCharacter.BP_FirstPersonCharacter_C|GetFireMode _returnvalue_10) 1)
    (Development|PrintString "1")
    ;[1 1 1] Fire linetrace for pistol
    (bind (_outhit _returnvalue_11) (Collision|LineTraceForObjects _returnvalue_2 (+ _returnvalue_2 (* (Math|Vector|GetForwardVector (Transformation|GetWorldRotation (Variables|Default|Getlinetrace))) (Variables|Pistol|GetlineTraceDistance))) (Utilities|Array|MakeArray "ObjectTypeQuery1" "ObjectTypeQuery2" "ObjectTypeQuery3") false (Utilities|Array|MakeArray self (Game|GetPlayerCharacter 0)) "ForDuration"))
    (if _returnvalue_11
      (Game|Damage|ApplyDamage (.HitActor (Collision|BreakHitResult _outhit)) (+ (Variables|Pistol|GetDMGpistol) (Math|Random|RandomInteger 10)) 0 0)
      (bind _returnvalue_12 (Actor|GetActorOfClass "/Game/FirstPerson/Blueprints/BP_FirstPersonCharacter.BP_FirstPersonCharacter_C"))
      (Variables|/Game/FirstPerson/Blueprints/BP_FirstPersonCharacter.BP_FirstPersonCharacter_C|SetBullets _returnvalue_12 (- (Variables|/Game/FirstPerson/Blueprints/BP_FirstPersonCharacter.BP_FirstPersonCharacter_C|GetBullets _returnvalue_12) 1)))
    (elif (== (Variables|/Game/FirstPerson/Blueprints/BP_FirstPersonCharacter.BP_FirstPersonCharacter_C|GetFireMode _returnvalue_10) 2)
      (Development|PrintString "2")
      ;[1 1 1] fire shotgun linetraces
      (if true
        (Utilities|FlowControl|DoOnce false :!label _label
          (:Completed
            (bind (_outhit_2 _returnvalue_13) (Collision|LineTraceForObjects (Transformation|GetWorldLocation (Variables|Default|Getlinetrace)) (Math|Vector|MakeVector (+ _x_2 (Math|Random|RandomFloatinRange _minspreadshotgun _maxspreadshotgun)) (+ _y_2 (Math|Random|RandomFloatinRange _minspreadshotgun _maxspreadshotgun)) (+ _z_2 (Math|Random|RandomFloatinRange _minspreadshotgun _maxspreadshotgun))) (Utilities|Array|MakeArray "ObjectTypeQuery1" "ObjectTypeQuery2" "ObjectTypeQuery3") false (Utilities|Array|MakeArray self (Game|GetPlayerCharacter 0)) "ForDuration" :!label _label_2))
            (if _returnvalue_13
              (Game|Damage|ApplyDamage (.HitActor (Collision|BreakHitResult _outhit_2)) (+ (Variables|Shotgun|GetDMGshotgun) (Math|Random|RandomInteger 5)) 0 0)
              ;;[1 1 1] controls ammount of Linetraces spawned per shot
              (Variables|Shotgun|SetTimesLooped (+ (Math|Random|RandomIntegerinRange 1 1) (Variables|Shotgun|GetTimesLooped)))
              (if (>= (Variables|Shotgun|GetTimesLooped) (Variables|Shotgun|GetShotgunBullets))
                (Variables|Shotgun|SetTimesLooped 0)
                (if true
                  (bind _returnvalue_14 (Actor|GetActorOfClass "/Game/FirstPerson/Blueprints/BP_FirstPersonCharacter.BP_FirstPersonCharacter_C"))
                  (Variables|/Game/FirstPerson/Blueprints/BP_FirstPersonCharacter.BP_FirstPersonCharacter_C|SetShells _returnvalue_14 (- (Variables|/Game/FirstPerson/Blueprints/BP_FirstPersonCharacter.BP_FirstPersonCharacter_C|GetShells _returnvalue_14) 1))
                  (Default|ShotgunJump _returnvalue_14)
                  (goto _label Reset))
                (else
                  (goto _label_2)))))))
      (elif (== (Variables|/Game/FirstPerson/Blueprints/BP_FirstPersonCharacter.BP_FirstPersonCharacter_C|GetFireMode _returnvalue_10) 3)
        (Development|PrintString "3")
        ;[1 1 1] Fire linetrace for machine gun
        (bind (_outhit_3 _returnvalue_15) (Collision|LineTraceForObjects (Transformation|GetWorldLocation (Variables|Default|Getlinetrace)) (Math|Vector|MakeVector (+ _x (Math|Random|RandomFloatinRange _minspreadmachinegun _maxspreadmachinegun)) (+ _y (Math|Random|RandomFloatinRange _minspreadmachinegun _maxspreadmachinegun)) (+ _z (Math|Random|RandomFloatinRange _minspreadmachinegun _maxspreadmachinegun))) (Utilities|Array|MakeArray "ObjectTypeQuery1" "ObjectTypeQuery2" "ObjectTypeQuery3") false (Utilities|Array|MakeArray self (Game|GetPlayerCharacter 0)) "ForDuration" :!label _label_3))
        (if _returnvalue_15
          (Game|Damage|ApplyDamage (.HitActor (Collision|BreakHitResult _outhit_3)) (+ (Variables|MachineGun|GetDMGmachinegun) (Math|Random|RandomInteger 12)) 0 0)
          ;;[1 1 1] controls ammount of Linetraces spawned per shot
          (Variables|MachineGun|SetTimesLoopedMachineGun (+ (Variables|MachineGun|GetTimesLoopedMachineGun) (Math|Random|RandomIntegerinRange 1 2)))
          (if (>= (Variables|MachineGun|GetTimesLoopedMachineGun) (Variables|MachineGun|GetMachineGunBullets))
            (Variables|MachineGun|SetTimesLoopedMachineGun 0)
            (if true
              (bind _returnvalue_16 (Actor|GetActorOfClass "/Game/FirstPerson/Blueprints/BP_FirstPersonCharacter.BP_FirstPersonCharacter_C"))
              (Variables|/Game/FirstPerson/Blueprints/BP_FirstPersonCharacter.BP_FirstPersonCharacter_C|SetBullets _returnvalue_16 (- (Variables|/Game/FirstPerson/Blueprints/BP_FirstPersonCharacter.BP_FirstPersonCharacter_C|GetBullets _returnvalue_16) 2))
              (Default|MachineGunGlide _returnvalue_16))
            (else
              (goto _label_3))))
        (elif (== (Variables|/Game/FirstPerson/Blueprints/BP_FirstPersonCharacter.BP_FirstPersonCharacter_C|GetFireMode _returnvalue_10) 4)
          (Development|PrintString "4"))))))