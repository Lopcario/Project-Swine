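; Rocket launcher weapon Blueprint with flipbook animation, built on a parent that supplies the FireWeapon call.
; ShootWeapon passes a DoOnce gate, plays the fire flipbook and a random sound, and turns on the first-person character's muzzle flash.
; FireWeapon runs only after the flipbook's length elapses, then the flash and animation return to idle.
; A short cooldown then calls ResetWeapon to reopen the gate; StopShooting is empty.
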(event Custom|Reset%20Weapon
  (bind _weaponflipbook (Variables|Default|GetWeaponflipbook))
  (Utilities|FlowControl|DoOnce false) ; enters at Reset
)

(event EventBeginPlay
  (|CallParentFunction))

(event Collision|EventActorBeginOverlap
  (params (OtherActor :type Actor%20Object%20Reference))
  (|CallParentFunction OtherActor) ; This node is disabled and will not be called.\nDrag off pins to build functionality.
)

(event EventTick
  (params (DeltaSeconds :type Float%20%28single-precision%29))
  (|CallParentFunction DeltaSeconds))

(event EventShootWeapon
  (bind _weaponflipbook (Variables|Default|GetWeaponflipbook))
  (Utilities|FlowControl|DoOnce false
    (:Completed
      (Sprite|SetFlipbook _weaponflipbook "/Game/Sprites/DevSpritesReplaceLater/RetroFPSAssets/Weapons/RPG/RPG_Fire.RPG_Fire")
      (bind _returnvalue (Actor|GetActorOfClass "/Game/FirstPerson/Blueprints/BP_FirstPersonCharacter.BP_FirstPersonCharacter_C"))
      (Default|MuzzleFlashon _returnvalue)
      (Audio|PlaySound2D (.OutItem (Utilities|Array|Random (Variables|Default|GetSound))) 1.0 1.0 0.0 0 0)
      (Utilities|FlowControl|Delay (Class|PaperFlipbookComponent|GetFlipbookLength _weaponflipbook))
      (CallFunction|FireWeapon)
      (Default|MuzzleFlashOff _returnvalue)
      (Sprite|SetFlipbook (Variables|Default|GetWeaponflipbook) "/Game/Sprites/DevSpritesReplaceLater/RetroFPSAssets/Weapons/RPG/RPG_Idle.RPG_Idle")
      (Utilities|FlowControl|Delay 0.6)
      (CallFunction|ResetWeapon))))

(event EventStopShooting)

(fn ConstructionScript
  (|CallParentFunction))