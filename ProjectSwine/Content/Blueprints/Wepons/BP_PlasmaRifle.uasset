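; Plasma rifle weapon Blueprint that fires a three-shot burst with flipbook sprite animation.
; ShootWeapon uses a DoOnce gate, turns on the player character's blue muzzle flash and plays a random 2D sound.
; Chained delays timed to the fire flipbook's length space the FireWeapon calls, with a wind-up before the first shot.
; It then returns to idle, switches the flash off and resets the gate; StopShooting is empty.
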(event Custom|Reset%20Weapon
  (bind _weaponflipbook (Variables|Default|GetWeaponflipbook))
  (bind _weaponflipbook_2 (Variables|Default|GetWeaponflipbook))
  (bind _weaponflipbook_3 (Variables|Default|GetWeaponflipbook))
  (bind _weaponflipbook_4 (Variables|Default|GetWeaponflipbook))
  (Utilities|FlowControl|DoOnce false) ; enters at Reset
)

(event EventBeginPlay
  (|CallParentFunction))

(event Collision|EventActorBeginOverlap
  (params (OtherActor :type Actor%20Object%20Reference))
  (|CallParentFunction OtherActor) ; This node is disabled and will not be called.\nDrag off pins to build functionality.
)

(event EventTick
  (params (DeltaSeconds :type Float%20%28single-precision%29))
  (|CallParentFunction DeltaSeconds))

(event EventShootWeapon
  (bind _weaponflipbook (Variables|Default|GetWeaponflipbook))
  (bind _weaponflipbook_2 (Variables|Default|GetWeaponflipbook))
  (bind _weaponflipbook_3 (Variables|Default|GetWeaponflipbook))
  (bind _weaponflipbook_4 (Variables|Default|GetWeaponflipbook))
  (Utilities|FlowControl|DoOnce false
    (:Completed
      (bind _returnvalue (Actor|GetActorOfClass "/Game/FirstPerson/Blueprints/BP_FirstPersonCharacter.BP_FirstPersonCharacter_C"))
      (Default|MuzzleFlashonBlue _returnvalue)
      (Sprite|SetFlipbook _weaponflipbook_2 "/Game/Sprites/DevSpritesReplaceLater/RetroFPSAssets/Weapons/PlasmaGun/FB_PlasmaRifleFire.FB_PlasmaRifleFire")
      (Audio|PlaySound2D (.OutItem (Utilities|Array|Random (Variables|Default|GetSound))) 0.5 1.0 0.0 0 0)
      (Utilities|FlowControl|Delay (Class|PaperFlipbookComponent|GetFlipbookLength _weaponflipbook_2))
      (Sprite|SetFlipbook _weaponflipbook_3 "/Game/Sprites/DevSpritesReplaceLater/RetroFPSAssets/Weapons/PlasmaGun/FB_PlasmaRifleFire.FB_PlasmaRifleFire")
      (Utilities|FlowControl|Delay (Class|PaperFlipbookComponent|GetFlipbookLength _weaponflipbook_3))
      (CallFunction|FireWeapon)
      (Sprite|SetFlipbook _weaponflipbook_4 "/Game/Sprites/DevSpritesReplaceLater/RetroFPSAssets/Weapons/PlasmaGun/FB_PlasmaRifleFire.FB_PlasmaRifleFire")
      (Utilities|FlowControl|Delay (Class|PaperFlipbookComponent|GetFlipbookLength _weaponflipbook_4))
      (CallFunction|FireWeapon)
      (Sprite|SetFlipbook _weaponflipbook "/Game/Sprites/DevSpritesReplaceLater/RetroFPSAssets/Weapons/PlasmaGun/FB_PlasmaRifleFire.FB_PlasmaRifleFire")
      (Utilities|FlowControl|Delay (Class|PaperFlipbookComponent|GetFlipbookLength _weaponflipbook))
      (CallFunction|FireWeapon)
      (Sprite|SetFlipbook (Variables|Default|GetWeaponflipbook) "/Game/Sprites/DevSpritesReplaceLater/RetroFPSAssets/Weapons/PlasmaGun/FB_PlasmaRifleIdle.FB_PlasmaRifleIdle")
      (Utilities|FlowControl|Delay 0.15)
      (bind _returnvalue_2 (Actor|GetActorOfClass "/Game/FirstPerson/Blueprints/BP_FirstPersonCharacter.BP_FirstPersonCharacter_C"))
      (Default|MuzzleFlashOffBlue _returnvalue_2)
      (CallFunction|ResetWeapon))))

(event EventStopShooting)

(fn ConstructionScript
  (|CallParentFunction))