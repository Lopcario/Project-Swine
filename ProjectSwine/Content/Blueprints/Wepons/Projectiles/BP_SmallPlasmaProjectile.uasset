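; Small plasma projectile Blueprint, drawn as a flipbook sprite that flies with random spread.
; BeginPlay sets local velocity with random Y/Z offsets, caches the player character and starts a self-calling delayed loop that yaws the sprite toward the player.
; The first Tick starts a timed self-destruct.
; SpawnBlood picks blood or a bullet hole by its own Enemy tag, but its only call is unconnected.
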(event Custom|Face%20Playerr
  ;[1 1 1] Forces sprite to face player
  (Transformation|SetActorRotation (Math|Rotator|MakeRotator 0.0 0.0 (.yaw (Math|Interpolation|RInterpTo (Transformation|GetActorRotation) (Math|Rotator|FindLookatRotation (Transformation|GetActorLocation) (Transformation|GetActorLocation (Variables|Default|GetCharRef))) (Utilities|Time|GetWorldDeltaSeconds) 2e+01))))
  (Utilities|FlowControl|Delay 0.001)
  (CallFunction|FacePlayerr))

(event Custom|SpawnBlood
  (bind _rocketidleflipbook (Variables|Default|GetRocketIdleFlipBook))
  (bind _returnvalue (Transformation|GetWorldTransform _rocketidleflipbook))
  (if (Actor|ActorHasTag "Enemy")
    (bind _returnvalue_2 (Game|SpawnActorfromClass "/Game/Blueprints/BloodNHoles/BloodEffect_BP.BloodEffect_BP_C" _returnvalue "Undefined" "MultiplyWithRoot" 0 0))
    (AddComponent|AddChildActorComponent _returnvalue_2 false)
    (else
      (Game|SpawnActorfromClass "/Game/Blueprints/BloodNHoles/BulletHole_BP1.BulletHole_BP1_C" _returnvalue "Undefined" "MultiplyWithRoot" 0 0))))

(event EventBeginPlay
  ;[1 1 1] Forces sprite to face player
  (Game|Components|ProjectileMovement|SetVelocityinLocalSpace (Variables|Default|GetProjectileMovement) (Math|Vector|MakeVector (Variables|Default|GetBullet%20Velocity%20X) (+ (Math|Random|RandomFloatinRange (Variables|Default|GetMinSpread) (Variables|Default|GetMaxSpread)) (Variables|Default|GetBullet%20Velocity%20Y)) (+ (Math|Random|RandomFloatinRange (Variables|Default|GetMinSpread) (Variables|Default|GetMaxSpread)) (Variables|Default|GetBullet%20Velocity%20Z))))
  (bind _asbp_first_person_character (Utilities|Casting|CastToBP_FirstPersonCharacter (Game|GetPlayerCharacter 0)))
  (Variables|Default|SetCharRef _asbp_first_person_character)
  (CallFunction|FacePlayerr))

(event EventTick
  (params (DeltaSeconds :type Float%20%28single-precision%29))
  (Utilities|FlowControl|DoOnce false
    (:Completed
      (Utilities|FlowControl|Delay 3.0)
      (Actor|DestroyActor))))

(fn ConstructionScript)

(fn FacePlayer)