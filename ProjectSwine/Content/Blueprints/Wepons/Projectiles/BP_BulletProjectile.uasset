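; BP_BulletProjectile is a short-lived bullet projectile whose sprite turns to face the player.
; BeginPlay sets its local velocity through ProjectileMovement, adding random spread on Y and Z, then caches the player character.
; FacePlayerr re-calls itself after a tiny delay, interpolating actor yaw toward the player, while the FacePlayer function is empty.
; Tick uses a DoOnce to start a brief delay that destroys the actor.
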(event Custom|Face%20Playerr
  ;[1 1 1] Forces sprite to face player
  (Transformation|SetActorRotation (Math|Rotator|MakeRotator 0.0 0.0 (.yaw (Math|Interpolation|RInterpTo (Transformation|GetActorRotation) (Math|Rotator|FindLookatRotation (Transformation|GetActorLocation) (Transformation|GetActorLocation (Variables|Default|GetCharRef))) (Utilities|Time|GetWorldDeltaSeconds) 2e+01))))
  (Utilities|FlowControl|Delay 0.001)
  (CallFunction|FacePlayerr))

(event EventBeginPlay
  ;[1 1 1] Forces sprite to face player
  (Game|Components|ProjectileMovement|SetVelocityinLocalSpace (Variables|Default|GetProjectileMovement) (Math|Vector|MakeVector (Variables|Default|GetBullet%20Velocity%20X) (+ (Math|Random|RandomFloatinRange (Variables|Default|GetMinSpread) (Variables|Default|GetMaxSpread)) (Variables|Default|GetBullet%20Velocity%20Y)) (+ (Math|Random|RandomFloatinRange (Variables|Default|GetMinSpread) (Variables|Default|GetMaxSpread)) (Variables|Default|GetBullet%20Velocity%20Z))))
  (bind _asbp_first_person_character (Utilities|Casting|CastToBP_FirstPersonCharacter (Game|GetPlayerCharacter 0)))
  (Variables|Default|SetCharRef _asbp_first_person_character)
  (CallFunction|FacePlayerr))

(event EventTick
  (params (DeltaSeconds :type Float%20%28single-precision%29))
  (Utilities|FlowControl|DoOnce false
    (:Completed
      (Utilities|FlowControl|Delay 0.5)
      (Actor|DestroyActor))))

(fn ConstructionScript)

(fn FacePlayer)