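; BP_BulletPuff is a short-lived flipbook effect actor that acts as a billboard bullet puff facing the player.
; On BeginPlay it caches the first-person character and starts a self-calling event with a tiny delay, used in place of Tick, that interpolates its yaw toward the player.
; It destroys itself once the flipbook's length has elapsed.
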(event Custom|FacePlayer2
  (Transformation|SetActorRotation (Math|Rotator|MakeRotator 0.0 0.0 (.yaw (Math|Interpolation|RInterpTo (Transformation|GetActorRotation) (Math|Rotator|FindLookatRotation (Transformation|GetActorLocation) (Transformation|GetActorLocation (Variables|Default|GetCharRef))) (Utilities|Time|GetWorldDeltaSeconds) 2e+01))))
  (Utilities|FlowControl|Delay 0.001)
  (CallFunction|FacePlayer2))

(event EventBeginPlay
  (bind _asbp_first_person_character (Utilities|Casting|CastToBP_FirstPersonCharacter (Game|GetPlayerCharacter 0)))
  (Variables|Default|SetCharRef _asbp_first_person_character)
  (CallFunction|FacePlayer2)
  (Utilities|FlowControl|Delay (Class|PaperFlipbookComponent|GetFlipbookLength (Variables|Default|GetBulletPuffFB)))
  (Actor|DestroyActor))

(event Collision|EventActorBeginOverlap
  (params (OtherActor :type Actor%20Object%20Reference)))

(event EventTick
  (params (DeltaSeconds :type Float%20%28single-precision%29)))

(fn ConstructionScript)

(fn FacePlayer)