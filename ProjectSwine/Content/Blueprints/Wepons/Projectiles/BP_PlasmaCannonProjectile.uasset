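; Plasma cannon projectile with a billboard flipbook sprite that explodes on overlap, damaging nearby non-player actors and scattering mini plasma balls.
; A self-repeating delayed event keeps its yaw turned toward the player.
; Overlap stops movement, then loops over every actor in the level to apply distance-checked damage, with explosion flipbook and sound triggered inside that loop.
; A DoOnce spawns twelve PlasmaBallMini actors, hides the light and destroys the projectile after the animation.
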(event OnComponentBeginOverlap(HitRadius)
  (params (OverlappedComponent :type Primitive%20Component%20Object%20Reference) (OtherActor :type Actor%20Object%20Reference) (OtherComp :type Primitive%20Component%20Object%20Reference) (OtherBodyIndex :type Integer) (bFromSweep :type Boolean) (SweepResult :type Hit%20Result%20Structure%20%28by%20ref%29))
  (bind _projectilemovement (Variables|Default|GetProjectileMovement))
  (bind _rocketidleflipbook (Variables|Default|GetRocketIdleFlipBook))
  (Variables|Default|SetOther%20Actor OtherActor)
  (if (Actor|ActorHasTag OtherActor "Player")
    _
    (else
      _))
  ;[1 1 1] Rocket Direct Damage
  (Variables|/Script/Engine.ProjectileMovementComponent|SetMaxSpeed _projectilemovement 0.0)
  (Variables|/Script/Engine.MovementComponent|SetVelocity _projectilemovement "0, 0, 0")
  ;[1 1 1] Rocket Explosion Damage
  (bind _outactors (Actor|GetAllActorsOfClass "/Script/Engine.Actor"))
  (for _array_element _outactors
    (bind _output_get (Variables|Default|SetActorInExplosionRange _array_element))
    (if (<= (Math|Vector|VectorLength (- (Transformation|GetActorLocation _array_element) (Transformation|GetActorLocation))) (Math|Float|MakeLiteralFloat (Variables|Default|GetExplosionRange)))
      (if (Actor|ActorHasTag _output_get "Player")
        _
        (else
          (Game|Damage|ApplyDamage (Variables|Default|GetActorInExplosionRange) (Math|Conversions|ToFloat(Integer) (Variables|Default|GetRocketExplosionDamage)) 0 0))))
    (Sprite|SetFlipbook _rocketidleflipbook "/Game/Sprites/DevSpritesReplaceLater/RetroFPSAssets/Projectiles/BFG/BFG.BFG")
    (Audio|PlaySound2D (.OutItem (Utilities|Array|Random (Variables|Default|GetExplosionSounds))) 0.1 1.0 0.0 0 0 false)
    (Utilities|FlowControl|DoOnce false
      (:Completed
        (Utilities|SpawnSmallPlasmaBalls
          (:out
            (Development|SetHiddeninGame (Variables|Default|GetPointLight) true false)
            (Utilities|FlowControl|Delay (Class|PaperFlipbookComponent|GetFlipbookLength _rocketidleflipbook))
            (Actor|DestroyActor)))))))

(event Custom|Face%20Playerr
  ;[1 1 1] Forces sprite to face player
  (Transformation|SetActorRotation (Math|Rotator|MakeRotator 0.0 0.0 (.yaw (Math|Interpolation|RInterpTo (Transformation|GetActorRotation) (Math|Rotator|FindLookatRotation (Transformation|GetActorLocation) (Transformation|GetActorLocation (Variables|Default|GetCharRef))) (Utilities|Time|GetWorldDeltaSeconds) 2e+01))))
  (Utilities|FlowControl|Delay 0.001)
  (CallFunction|FacePlayerr))

(event EventBeginPlay
  ;[1 1 1] Forces sprite to face player
  (bind _asbp_first_person_character (Utilities|Casting|CastToBP_FirstPersonCharacter (Game|GetPlayerCharacter 0)))
  (Variables|Default|SetCharRef _asbp_first_person_character)
  (CallFunction|FacePlayerr))

(fn ConstructionScript)

(fn FacePlayer)