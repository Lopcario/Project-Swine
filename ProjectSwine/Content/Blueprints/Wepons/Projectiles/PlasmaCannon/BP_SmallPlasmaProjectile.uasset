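; Small plasma cannon projectile, drawn as a flipbook sprite that yaws toward the player through a self-repeating delayed event.
; BeginPlay launches it with random lateral and vertical spread.
; Tick drops lingering plasma actors behind it and times out into the BFG flipbook before destruction.
; Overlapping anything not tagged Player or Projectile damages non-player actors within explosion range, found by scanning all actors, then plays that flipbook and destroys it.
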(event OnComponentBeginOverlap(HitBox)
  (params (OverlappedComponent :type Primitive%20Component%20Object%20Reference) (OtherActor :type Actor%20Object%20Reference) (OtherComp :type Primitive%20Component%20Object%20Reference) (OtherBodyIndex :type Integer) (bFromSweep :type Boolean) (SweepResult :type Hit%20Result%20Structure%20%28by%20ref%29))
  (bind _rocketidleflipbook (Variables|Default|GetRocketIdleFlipBook))
  (Variables|Default|SetOther%20Actor OtherActor)
  (if (not (Actor|ActorHasTag OtherActor "Player"))
    (if (not (Actor|ActorHasTag OtherActor "Projectile"))
      (bind _outactors (Actor|GetAllActorsOfClass "/Script/Engine.Actor"))
      (for _array_element _outactors
        (bind _output_get (Variables|Default|SetActorInExplosionRange _array_element))
        (if (<= (Math|Vector|VectorLength (- (Transformation|GetActorLocation _array_element) (Transformation|GetActorLocation))) (Math|Float|MakeLiteralFloat (Variables|Default|GetExplosionRange)))
          (if (Actor|ActorHasTag _output_get "Player")
            _
            (else
              (Game|Damage|ApplyDamage (Variables|Default|GetActorInExplosionRange) (Math|Conversions|ToFloat(Integer) (Variables|Default|GetPlasmaExplosionDamage)) 0 0))))
        (Sprite|SetFlipbook _rocketidleflipbook "/Game/Sprites/CustomSprites/Projectiles/BFG/BFG.BFG")
        (Utilities|FlowControl|Delay (Class|PaperFlipbookComponent|GetFlipbookLength _rocketidleflipbook))
        (Actor|DestroyActor)))))

(event Custom|Face%20Playerr
  ;[1 1 1] Forces sprite to face player
  (Transformation|SetActorRotation (Math|Rotator|MakeRotator 0.0 0.0 (.yaw (Math|Interpolation|RInterpTo (Transformation|GetActorRotation) (Math|Rotator|FindLookatRotation (Transformation|GetActorLocation) (Transformation|GetActorLocation (Variables|Default|GetCharRef))) (Utilities|Time|GetWorldDeltaSeconds) 2e+01))))
  (Utilities|FlowControl|Delay 0.001)
  (CallFunction|FacePlayerr))

(event EventBeginPlay
  ;[1 1 1] Forces sprite to face player
  (Game|Components|ProjectileMovement|SetVelocityinLocalSpace (Variables|Default|GetProjectileMovement) (Math|Vector|MakeVector (Variables|Default|GetBullet%20Velocity%20X) (+ (Math|Random|RandomFloatinRange (Variables|Default|GetMinSpread) (Variables|Default|GetMaxSpread)) (Variables|Default|GetBullet%20Velocity%20Y)) (+ (Math|Random|RandomFloatinRange (Variables|Default|GetMinSpreadZ) (Variables|Default|GetMaxSpreadZ)) (Variables|Default|GetBullet%20Velocity%20Z))))
  (bind _asbp_first_person_character (Utilities|Casting|CastToBP_FirstPersonCharacter (Game|GetPlayerCharacter 0)))
  (Variables|Default|SetCharRef _asbp_first_person_character)
  (CallFunction|FacePlayerr))

(event EventTick
  (params (DeltaSeconds :type Float%20%28single-precision%29))
  (bind _rocketidleflipbook (Variables|Default|GetRocketIdleFlipBook))
  (Utilities|FlowControl|Delay 0.07)
  (Game|SpawnActorfromClass "/Game/Blueprints/Wepons/Projectiles/PlasmaCannon/BP_SmallPlasmaLingering.BP_SmallPlasmaLingering_C" (Transformation|GetWorldTransform (Variables|Default|GetRocketIdleFlipBook)) "Undefined" "MultiplyWithRoot" 0 0)
  (Utilities|FlowControl|DoOnce false
    (:Completed
      (Utilities|FlowControl|Delay 1.0)
      (Sprite|SetFlipbook _rocketidleflipbook "/Game/Sprites/CustomSprites/Projectiles/BFG/BFG.BFG")
      (Utilities|FlowControl|Delay (Class|PaperFlipbookComponent|GetFlipbookLength _rocketidleflipbook))
      (Actor|DestroyActor))))

(fn ConstructionScript)

(fn FacePlayer)