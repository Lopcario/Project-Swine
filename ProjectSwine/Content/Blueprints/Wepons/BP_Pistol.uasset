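; Pistol weapon Blueprint that fires single shots with flipbook animation, muzzle flash and sound.
; ShootWeapon passes a DoOnce gate, calls FireWeapon, plays the fire flipbook, turns on the first-person character's muzzle flash, and plays a random sound with varied pitch.
; A delay matching the flipbook length then turns off the flash, restores the idle flipbook and calls ResetWeapon to reopen the gate.
; StopShooting is empty.
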(event Custom|Reset%20Weapon
  (bind _weaponflipbook (Variables|Default|GetWeaponflipbook))
  (Utilities|FlowControl|DoOnce false) ; enters at Reset
)

(event EventBeginPlay
  (|CallParentFunction) ; This node is disabled and will not be called.\nDrag off pins to build functionality.
)

(event Collision|EventActorBeginOverlap
  (params (OtherActor :type Actor%20Object%20Reference))
  (|CallParentFunction OtherActor) ; This node is disabled and will not be called.\nDrag off pins to build functionality.
)

(event EventTick
  (params (DeltaSeconds :type Float%20%28single-precision%29))
  (|CallParentFunction DeltaSeconds) ; This node is disabled and will not be called.\nDrag off pins to build functionality.
)

(event EventShootWeapon
  (bind _weaponflipbook (Variables|Default|GetWeaponflipbook))
  (Utilities|FlowControl|DoOnce false
    (:Completed
      (CallFunction|FireWeapon)
      (Sprite|SetFlipbook _weaponflipbook "/Game/Sprites/DevSpritesReplaceLater/RetroFPSAssets/Weapons/Pistol/PistolFire.PistolFire")
      (bind _returnvalue (Actor|GetActorOfClass "/Game/FirstPerson/Blueprints/BP_FirstPersonCharacter.BP_FirstPersonCharacter_C"))
      (Default|MuzzleFlashon _returnvalue)
      (Audio|PlaySound2D (.OutItem (Utilities|Array|Random (Variables|Default|GetSound))) 0.8 (Math|Random|RandomFloatinRange 0.8 1.2) 0.0 0 0)
      (Utilities|FlowControl|Delay (Class|PaperFlipbookComponent|GetFlipbookLength _weaponflipbook))
      (Default|MuzzleFlashOff _returnvalue)
      (Sprite|SetFlipbook (Variables|Default|GetWeaponflipbook) "/Game/Sprites/DevSpritesReplaceLater/RetroFPSAssets/Weapons/Pistol/PistolIdle.PistolIdle")
      (CallFunction|ResetWeapon))))

(event EventStopShooting)

(fn ConstructionScript
  (|CallParentFunction))