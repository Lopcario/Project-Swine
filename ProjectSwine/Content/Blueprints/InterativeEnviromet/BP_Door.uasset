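; BP_Door is a color-coded keycard door that opens once the player holds the matching blue, orange or red key.
; On BeginPlay, KeyCardColor swaps both door sprites to orange or red, leaving blue as the unset default.
; Tick polls the first-person character's key flags with no proximity check.
; A match fires a shared DoOnce that plays a sound and slides the door mesh to the OpendoorVisual position.
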(event EventBeginPlay
  (bind _bluedoor_sprite1 (Variables|Default|Getbluedoor_Sprite1))
  (bind _bluedoor_sprite (Variables|Default|Getbluedoor_Sprite))
  (if (not (== (Variables|Default|GetKeyCardColor) 1))
    (if (== (Variables|Default|GetKeyCardColor) 2)
      (Rendering|Components|Sprite|SetSprite _bluedoor_sprite1 "/Game/Sprites/CustomSprites/Pickups/Orangedoor_Sprite.Orangedoor_Sprite")
      (Rendering|Components|Sprite|SetSprite _bluedoor_sprite "/Game/Sprites/CustomSprites/Pickups/Orangedoor_Sprite.Orangedoor_Sprite")
      (elif (== (Variables|Default|GetKeyCardColor) 3)
        (Rendering|Components|Sprite|SetSprite _bluedoor_sprite1 "/Game/Sprites/CustomSprites/Pickups/reddoor_Sprite.reddoor_Sprite")
        (Rendering|Components|Sprite|SetSprite _bluedoor_sprite "/Game/Sprites/CustomSprites/Pickups/reddoor_Sprite.reddoor_Sprite")))))

(event Collision|EventActorBeginOverlap
  (params (OtherActor :type Actor%20Object%20Reference)))

(event EventTick
  (params (DeltaSeconds :type Float%20%28single-precision%29))
  (if (== (Variables|Default|GetKeyCardColor) 1)
    (bind _asbp_first_person_character (Utilities|Casting|CastToBP_FirstPersonCharacter (Game|GetPlayerCharacter 0)))
    (if (Variables|/Game/FirstPerson/Blueprints/BP_FirstPersonCharacter.BP_FirstPersonCharacter_C|GetHasBlueKey _asbp_first_person_character)
      (Utilities|FlowControl|DoOnce false :!label _label
        (:Completed
          (Audio|PlaySound2D "/Game/sounds/q009/jumppad2.jumppad2" 1.0 1.0 0.0 0 0)
          (Components|MoveComponentTo (Variables|Default|GetDoorFBX) (Variables|/Script/Engine.SceneComponent|GetRelativeLocation (Variables|Default|GetOpendoorVisual)) "0, 0, 0" false false 0.5 false))))
    (elif (== (Variables|Default|GetKeyCardColor) 2)
      (bind _asbp_first_person_character_2 (Utilities|Casting|CastToBP_FirstPersonCharacter (Game|GetPlayerCharacter 0)))
      (if (Variables|/Game/FirstPerson/Blueprints/BP_FirstPersonCharacter.BP_FirstPersonCharacter_C|GetHasOrangeKey _asbp_first_person_character_2)
        (goto _label))
      (elif (== (Variables|Default|GetKeyCardColor) 3)
        (bind _asbp_first_person_character_3 (Utilities|Casting|CastToBP_FirstPersonCharacter (Game|GetPlayerCharacter 0)))
        (if (Variables|/Game/FirstPerson/Blueprints/BP_FirstPersonCharacter.BP_FirstPersonCharacter_C|GetHasRedKey _asbp_first_person_character_3)
          (goto _label))))))

(fn ConstructionScript)