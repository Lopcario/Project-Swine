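; Elevator actor that slides its DoorFBX mesh between start (down) and open (up) locations with a sound, initially placed according to StartHigh.
; Tick polls the first-person character's Trigger flags against TriggerNumber for a one-shot move; the Trigger4 branch checks number 1, and slots 6–10 compare constants.
; With AutoElvator set, Player or Enemy overlap moves it, and exit reverses it after a delay, then calls Resett, which also runs GoUp.
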(event OnComponentBeginOverlap(DoorTrigger)
  (params (OverlappedComponent :type Primitive%20Component%20Object%20Reference) (OtherActor :type Actor%20Object%20Reference) (OtherComp :type Primitive%20Component%20Object%20Reference) (OtherBodyIndex :type Integer) (bFromSweep :type Boolean) (SweepResult :type Hit%20Result%20Structure%20%28by%20ref%29))
  (Variables|Default|SetOther%20Actor OtherActor)
  (if (Variables|Default|GetAutoElvator)
    (if (Variables|Default|GetStartHigh)
      (if (or (Actor|ActorHasTag (Variables|Default|GetOther%20Actor) "Player") (Actor|ActorHasTag (Variables|Default|GetOther%20Actor) "Enemy"))
        (CallFunction|GoDown))
      (elif (or (Actor|ActorHasTag (Variables|Default|GetOther%20Actor) "Player") (Actor|ActorHasTag (Variables|Default|GetOther%20Actor) "Enemy"))
        (CallFunction|GoUp)))))

(event OnComponentEndOverlap(DoorTrigger)
  (params (OverlappedComponent :type Primitive%20Component%20Object%20Reference) (OtherActor :type Actor%20Object%20Reference) (OtherComp :type Primitive%20Component%20Object%20Reference) (OtherBodyIndex :type Integer))
  (Variables|Default|SetOther%20Actor OtherActor)
  (if (Variables|Default|GetAutoElvator)
    (if (Variables|Default|GetStartHigh)
      (if (or (Actor|ActorHasTag (Variables|Default|GetOther%20Actor) "Player") (Actor|ActorHasTag (Variables|Default|GetOther%20Actor) "Enemy"))
        (Utilities|FlowControl|Delay 4.0)
        (CallFunction|GoUp)
        (Utilities|FlowControl|Delay 5.0)
        (CallFunction|Resett))
      (elif (or (Actor|ActorHasTag (Variables|Default|GetOther%20Actor) "Player") (Actor|ActorHasTag (Variables|Default|GetOther%20Actor) "Enemy"))
        (Utilities|FlowControl|Delay 4.0)
        (CallFunction|GoDown)
        (Utilities|FlowControl|Delay 5.0)
        (CallFunction|Resett)))))

(event Custom|GoUp
  ;[1 1 1] Opens Door
  (Utilities|FlowControl|DoOnce false :!label _label
    (:Completed
      (Utilities|FlowControl|Delay 1.0)
      (Audio|PlaySound2D "/Game/sounds/q009/jumppad2.jumppad2" 1.0 1.0 0.0 0 0)
      (Components|MoveComponentTo (Variables|Default|GetDoorFBX) (Variables|/Script/Engine.SceneComponent|GetRelativeLocation (Variables|Default|GetDoorOpenLocation)) "0, 0, 0" false false 2.0 false)
      (Utilities|FlowControl|Delay 1.0)
      (goto _label Reset))))

(event Custom|GoDown
  ;[1 1 1] Close door
  (Utilities|FlowControl|DoOnce false :!label _label
    (:Completed
      (Audio|PlaySound2D "/Game/sounds/q009/jumppad2.jumppad2" 1.0 1.0 0.0 0 0)
      (Components|MoveComponentTo (Variables|Default|GetDoorFBX) (Variables|/Script/Engine.SceneComponent|GetRelativeLocation (Variables|Default|GetDoorStartLocation)) "0, 0, 0" false false 2.0 false)
      (Utilities|FlowControl|Delay 1.0)
      (goto _label Reset))))

(event Custom|Resett
  (Utilities|FlowControl|DoOnce false ; enters at Reset
    (:Completed
      (CallFunction|GoUp))))

(event EventBeginPlay
  (if (Variables|Default|GetStartHigh)
    (Components|MoveComponentTo (Variables|Default|GetDoorFBX) (Variables|/Script/Engine.SceneComponent|GetRelativeLocation (Variables|Default|GetDoorOpenLocation)) "0, 0, 0" false false 2.0 false)
    (else
      (Components|MoveComponentTo (Variables|Default|GetDoorFBX) (Variables|/Script/Engine.SceneComponent|GetRelativeLocation (Variables|Default|GetDoorStartLocation)) "0, 0, 0" false false 2.0 false))))

(event Collision|EventActorBeginOverlap
  (params (OtherActor :type Actor%20Object%20Reference)))

(event EventTick
  (params (DeltaSeconds :type Float%20%28single-precision%29))
  (bind _returnvalue (Actor|GetActorOfClass "/Game/FirstPerson/Blueprints/BP_FirstPersonCharacter.BP_FirstPersonCharacter_C"))
  (if (and (== (Variables|Default|GetTriggerNumber) 1) (Variables|/Game/FirstPerson/Blueprints/BP_FirstPersonCharacter.BP_FirstPersonCharacter_C|GetTrigger1 _returnvalue))
    (if (Variables|Default|GetStartHigh) :!label _label
      (Utilities|FlowControl|DoOnce false
        (:Completed
          (CallFunction|GoDown)))
      (else
        (Utilities|FlowControl|DoOnce false
          (:Completed
            (CallFunction|GoUp)))))
    (elif (and (== (Variables|Default|GetTriggerNumber) 2) (Variables|/Game/FirstPerson/Blueprints/BP_FirstPersonCharacter.BP_FirstPersonCharacter_C|GetTrigger2 _returnvalue))
      (goto _label)
      (elif (and (== (Variables|Default|GetTriggerNumber) 3) (Variables|/Game/FirstPerson/Blueprints/BP_FirstPersonCharacter.BP_FirstPersonCharacter_C|GetTrigger3 _returnvalue))
        (goto _label)
        (elif (and (== (Variables|Default|GetTriggerNumber) 1) (Variables|/Game/FirstPerson/Blueprints/BP_FirstPersonCharacter.BP_FirstPersonCharacter_C|GetTrigger4 _returnvalue))
          (goto _label)
          (elif (and (== (Variables|Default|GetTriggerNumber) 5) (Variables|/Game/FirstPerson/Blueprints/BP_FirstPersonCharacter.BP_FirstPersonCharacter_C|GetTrigger5 _returnvalue))
            (goto _label)
            (elif (== 0 6)
              (goto _label)
              (elif (== 0 7)
                (goto _label)
                (elif (== 0 8)
                  (goto _label)
                  (elif (== 0 9)
                    (goto _label)
                    (elif (== 0 10)
                      (goto _label))))))))))))

(fn ConstructionScript)