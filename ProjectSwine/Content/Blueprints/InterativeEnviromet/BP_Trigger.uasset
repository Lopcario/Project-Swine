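; BP_Trigger is a one-shot trigger volume that notifies the first-person character when the player enters it.
; Its Box overlap sets HasBeenTriggered for any actor tagged Player.
; Tick polls that flag and, through a DoOnce, prints a debug "Hello", then finds BP_FirstPersonCharacter by class and calls its Triggers with this instance's TriggerNumber.
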(event OnComponentBeginOverlap(Box)
  (params (OverlappedComponent :type Primitive%20Component%20Object%20Reference) (OtherActor :type Actor%20Object%20Reference) (OtherComp :type Primitive%20Component%20Object%20Reference) (OtherBodyIndex :type Integer) (bFromSweep :type Boolean) (SweepResult :type Hit%20Result%20Structure%20%28by%20ref%29))
  (if (Actor|ActorHasTag OtherActor "Player")
    (Variables|Default|SetHasBeenTriggered true)))

(event EventTick
  (params (DeltaSeconds :type Float%20%28single-precision%29))
  (if (Variables|Default|GetHasBeenTriggered)
    (Utilities|FlowControl|DoOnce false
      (:Completed
        (Development|PrintString "Hello")
        (bind _returnvalue (Actor|GetActorOfClass "/Game/FirstPerson/Blueprints/BP_FirstPersonCharacter.BP_FirstPersonCharacter_C"))
        (Default|Triggers _returnvalue (Variables|Default|GetTriggerNumber))))))

(fn ConstructionScript)