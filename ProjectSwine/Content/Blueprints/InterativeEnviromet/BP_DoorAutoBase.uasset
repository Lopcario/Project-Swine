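; Base automatic door that slides its mesh between start and open locations with a sound.
; When ActivatedByTrigger, Tick matches TriggerNumber to the player's Trigger flags and opens once; slot 4 tests number 1, and 6-10 are dead checks.
; Otherwise Tick opens it when the nearby player is activating something, then closes it after a delay.
; Enemy overlap opens doors flagged IsDoor and exit closes them after a delay, while player overlap only sets PlayerIsByDoor.
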(event OnComponentBeginOverlap(DoorTrigger)
  (params (OverlappedComponent :type Primitive%20Component%20Object%20Reference) (OtherActor :type Actor%20Object%20Reference) (OtherComp :type Primitive%20Component%20Object%20Reference) (OtherBodyIndex :type Integer) (bFromSweep :type Boolean) (SweepResult :type Hit%20Result%20Structure%20%28by%20ref%29))
  (Variables|Default|SetOther%20Actor OtherActor)
  (if (Variables|Default|GetIsDoor)
    (if (or (Actor|ActorHasTag (Variables|Default|GetOther%20Actor) "Player") (Actor|ActorHasTag (Variables|Default|GetOther%20Actor) "Enemy"))
      (if (Actor|ActorHasTag (Variables|Default|GetOther%20Actor) "Player")
        (Variables|Default|SetPlayerIsByDoor true)
        (else
          (CallFunction|OpenDoor))))))

(event OnComponentEndOverlap(DoorTrigger)
  (params (OverlappedComponent :type Primitive%20Component%20Object%20Reference) (OtherActor :type Actor%20Object%20Reference) (OtherComp :type Primitive%20Component%20Object%20Reference) (OtherBodyIndex :type Integer))
  (Variables|Default|SetOther%20Actor OtherActor)
  (if (Actor|ActorHasTag (Variables|Default|GetOther%20Actor) "Enemy")
    (if (Actor|ActorHasTag (Variables|Default|GetOther%20Actor) "Enemy")
      (Utilities|FlowControl|Delay 3.0)
      (CallFunction|CloseDoor)
      (else
        (Variables|Default|SetPlayerIsByDoor false)))))

(event Custom|OpenDoor
  ;[1 1 1] Opens Door
  (Utilities|FlowControl|DoOnce false :!label _label
    (:Completed
      (Audio|PlaySound2D "/Game/sounds/q009/jumppad2.jumppad2" 1.0 1.0 0.0 0 0)
      (Components|MoveComponentTo (Variables|Default|GetDoorFBX) (Variables|/Script/Engine.SceneComponent|GetRelativeLocation (Variables|Default|GetDoorOpenLocation)) "0, 0, 0" true false 1.0 false)
      (Utilities|FlowControl|Delay 1.0)
      (goto _label Reset))))

(event Custom|CloseDoor
  ;[1 1 1] Close door
  (Utilities|FlowControl|DoOnce false :!label _label
    (:Completed
      (Audio|PlaySound2D "/Game/sounds/q009/jumppad2.jumppad2" 1.0 1.0 0.0 0 0)
      (Components|MoveComponentTo (Variables|Default|GetDoorFBX) (Variables|/Script/Engine.SceneComponent|GetRelativeLocation (Variables|Default|GetDoorStartLocation)) "0, 0, 0" false true 1.0 false)
      (Utilities|FlowControl|Delay 1.0)
      (goto _label Reset))))

(event EventBeginPlay)

(event Collision|EventActorBeginOverlap
  (params (OtherActor :type Actor%20Object%20Reference)))

(event EventTick
  (params (DeltaSeconds :type Float%20%28single-precision%29))
  (if (Variables|Default|GetActivatedByTrigger)
    (bind _returnvalue (Actor|GetActorOfClass "/Game/FirstPerson/Blueprints/BP_FirstPersonCharacter.BP_FirstPersonCharacter_C"))
    (if (and (== (Variables|Default|GetTriggerNumber) 1) (Variables|/Game/FirstPerson/Blueprints/BP_FirstPersonCharacter.BP_FirstPersonCharacter_C|GetTrigger1 _returnvalue))
      (if true :!label _label
        _
        (else
          _))
      (Utilities|FlowControl|DoOnce false
        (:Completed
          (CallFunction|OpenDoor)))
      (elif (and (== (Variables|Default|GetTriggerNumber) 2) (Variables|/Game/FirstPerson/Blueprints/BP_FirstPersonCharacter.BP_FirstPersonCharacter_C|GetTrigger2 _returnvalue))
        (goto _label)
        (elif (and (== (Variables|Default|GetTriggerNumber) 3) (Variables|/Game/FirstPerson/Blueprints/BP_FirstPersonCharacter.BP_FirstPersonCharacter_C|GetTrigger3 _returnvalue))
          (goto _label)
          (elif (and (== (Variables|Default|GetTriggerNumber) 1) (Variables|/Game/FirstPerson/Blueprints/BP_FirstPersonCharacter.BP_FirstPersonCharacter_C|GetTrigger4 _returnvalue))
            (goto _label)
            (elif (and (== (Variables|Default|GetTriggerNumber) 5) (Variables|/Game/FirstPerson/Blueprints/BP_FirstPersonCharacter.BP_FirstPersonCharacter_C|GetTrigger5 _returnvalue))
              (goto _label)
              (elif (== 0 6)
                (goto _label)
                (elif (== 0 7)
                  (goto _label)
                  (elif (== 0 8)
                    (goto _label)
                    (elif (== 0 9)
                      (goto _label)
                      (elif (== 0 10)
                        (goto _label)))))))))))
    (else
      (bind _returnvalue_2 (Actor|GetActorOfClass "/Game/FirstPerson/Blueprints/BP_FirstPersonCharacter.BP_FirstPersonCharacter_C"))
      (if (Variables|/Game/FirstPerson/Blueprints/BP_FirstPersonCharacter.BP_FirstPersonCharacter_C|GetIsActivatingSomething _returnvalue_2)
        (if (<= (Math|Vector|Distance(Vector) (Transformation|GetWorldLocation (Variables|Default|GetDoorTrigger)) (Transformation|GetWorldLocation (Variables|/Script/Engine.Character|GetCapsuleComponent _returnvalue_2))) 1.5e+02)
          (Utilities|FlowControl|DoOnce false :!label _label_2
            (:Completed
              (CallFunction|OpenDoor)
              (Utilities|FlowControl|Delay 3.0)
              (CallFunction|CloseDoor)
              (goto _label_2 Reset))))))))

(event Input|KeyboardEvents|E
  (params (Key :type Key%20Structure :default "None")))

(fn ConstructionScript)