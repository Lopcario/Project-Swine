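; BP_Switch is a one-shot interactive switch that the player activates at close range.
; Until triggered, it polls every Tick for BP_FirstPersonCharacter and checks that the character is activating something within 150 units of the switch's origin component.
; On activation it locks itself, swaps its sprite to the switched image and passes its TriggerNumber to the character's Triggers function.
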(event EventBeginPlay)

(event Collision|EventActorBeginOverlap
  (params (OtherActor :type Actor%20Object%20Reference)))

(event EventTick
  (params (DeltaSeconds :type Float%20%28single-precision%29))
  (if (not (Variables|Default|GetHasBeenTriggered))
    (bind _returnvalue (Actor|GetActorOfClass "/Game/FirstPerson/Blueprints/BP_FirstPersonCharacter.BP_FirstPersonCharacter_C"))
    (if (Variables|/Game/FirstPerson/Blueprints/BP_FirstPersonCharacter.BP_FirstPersonCharacter_C|GetIsActivatingSomething _returnvalue)
      (if (<= (Math|Vector|Distance(Vector) (Transformation|GetWorldLocation (Variables|Default|GetOrgin)) (Transformation|GetWorldLocation (Variables|/Script/Engine.Character|GetCapsuleComponent _returnvalue))) 1.5e+02)
        (Variables|Default|SetHasBeenTriggered true)
        (Rendering|Components|Sprite|SetSprite (Variables|Default|Getsw3s0_Sprite) "/Game/Sprites/CustomSprites/sprites/Sprite2/sw3s1_Sprite.sw3s1_Sprite")
        (bind _returnvalue_2 (Actor|GetActorOfClass "/Game/FirstPerson/Blueprints/BP_FirstPersonCharacter.BP_FirstPersonCharacter_C"))
        (Default|Triggers _returnvalue_2 (Variables|Default|GetTriggerNumber))))))

(fn ConstructionScript)