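; Enemy melee attack projectile that deals randomized radial damage to the player, apparently adapted from a fireball/rocket projectile.
; HitBox overlaps ignore the spawner and Projectile or Pickup actors, then scan all actors by distance once, damaging only the tagged player.
; The scan also plays quiet random impact sounds, including for out-of-range actors, and destroys the projectile after a short delay.
; Sprite-facing, spawn sound and explosion flipbook logic are disconnected.
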(event OnComponentBeginOverlap(HitRadius)
  (params (OverlappedComponent :type Primitive%20Component%20Object%20Reference) (OtherActor :type Actor%20Object%20Reference) (OtherComp :type Primitive%20Component%20Object%20Reference) (OtherBodyIndex :type Integer) (bFromSweep :type Boolean) (SweepResult :type Hit%20Result%20Structure%20%28by%20ref%29)))

(event OnComponentBeginOverlap(HitBox)
  (params (OverlappedComponent :type Primitive%20Component%20Object%20Reference) (OtherActor :type Actor%20Object%20Reference) (OtherComp :type Primitive%20Component%20Object%20Reference) (OtherBodyIndex :type Integer) (bFromSweep :type Boolean) (SweepResult :type Hit%20Result%20Structure%20%28by%20ref%29))
  (Utilities|FlowControl|Delay 0.001)
  (Variables|Default|SetOther%20Actor OtherActor)
  (if (not (== OtherActor (Variables|Default|GetActorThatSpawnedSelf)))
    (if (not (Math|Boolean|ORBoolean (Actor|ActorHasTag (Variables|Default|GetOther%20Actor) "Projectile") (Actor|ActorHasTag (Variables|Default|GetOther%20Actor) "Pickup") false))
      (Utilities|FlowControl|DoOnce false
        (:Completed
          ;[1 1 1] Rocket Explosion Damage
          (bind _outactors (Actor|GetAllActorsOfClass "/Script/Engine.Actor"))
          (for _array_element _outactors
            (bind _output_get (Variables|Default|SetActorInExplosionRange _array_element))
            (if (<= (Math|Vector|VectorLength (- (Transformation|GetActorLocation _array_element) (Transformation|GetActorLocation))) (Math|Float|MakeLiteralFloat (Variables|Default|GetFireballExplosionRange)))
              (if (Actor|ActorHasTag _output_get "Player")
                (bind _returnvalue (Actor|GetActorOfClass "/Game/FirstPerson/Blueprints/BP_FirstPersonCharacter.BP_FirstPersonCharacter_C"))
                (Default|TakeDamage _returnvalue (Math|Conversions|ToFloat(Integer) (+ (Variables|Default|GetFireballExplosionDamage) (* 3 (Math|Random|RandomIntegerinRange 0 7)))))
                (Audio|PlaySound2D (.OutItem (Utilities|Array|Random (Variables|Default|GetExplosionSounds))) 0.01 1.0 0.0 0 0 false :!label _label)
                (Utilities|FlowControl|DoOnce false
                  (:Completed
                    (Utilities|FlowControl|Delay 0.5)
                    (Actor|DestroyActor))))
              (else
                (goto _label)))))))))

(event Custom|Face%20Playerr
  ;[1 1 1] Forces sprite to face player
  (Transformation|SetActorRotation (Math|Rotator|MakeRotator 0.0 0.0 (.yaw (Math|Interpolation|RInterpTo (Transformation|GetActorRotation) (Math|Rotator|FindLookatRotation (Transformation|GetActorLocation) (Transformation|GetActorLocation (Variables|Default|GetCharRef))) (Utilities|Time|GetWorldDeltaSeconds) 2e+01))))
  (Utilities|FlowControl|Delay 0.001)
  (CallFunction|FacePlayerr))

(event EventBeginPlay
  ;[1 1 1] Forces sprite to face player
  (bind _asbp_first_person_character (Utilities|Casting|CastToBP_FirstPersonCharacter (Game|GetPlayerCharacter 0)))
  (Variables|Default|SetCharRef _asbp_first_person_character))

(fn ConstructionScript)

(fn FacePlayer)