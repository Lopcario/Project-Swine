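; BP_DoorAutoBase is an automatic sliding door that opens for actors tagged Player or Enemy.
; When IsDoor is set, entering DoorTrigger opens it and leaving starts a three-second delay before closing.
; Opening and closing play a 2D sound and ease DoorSprite between the relative locations of DoorOpenLocation and DoorStartLocation using MoveComponentTo.
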(event OnComponentBeginOverlap(DoorTrigger)
  (params (OverlappedComponent :type Primitive%20Component%20Object%20Reference) (OtherActor :type Actor%20Object%20Reference) (OtherComp :type Primitive%20Component%20Object%20Reference) (OtherBodyIndex :type Integer) (bFromSweep :type Boolean) (SweepResult :type Hit%20Result%20Structure%20%28by%20ref%29))
  (Variables|Default|SetOther%20Actor OtherActor)
  (if (Variables|Default|GetIsDoor)
    (if (or (Actor|ActorHasTag (Variables|Default|GetOther%20Actor) "Player") (Actor|ActorHasTag (Variables|Default|GetOther%20Actor) "Enemy"))
      (CallFunction|OpenDoor))))

(event OnComponentEndOverlap(DoorTrigger)
  (params (OverlappedComponent :type Primitive%20Component%20Object%20Reference) (OtherActor :type Actor%20Object%20Reference) (OtherComp :type Primitive%20Component%20Object%20Reference) (OtherBodyIndex :type Integer))
  (Variables|Default|SetOther%20Actor OtherActor)
  (if (Variables|Default|GetIsDoor)
    (if (or (Actor|ActorHasTag (Variables|Default|GetOther%20Actor) "Player") (Actor|ActorHasTag (Variables|Default|GetOther%20Actor) "Enemy"))
      (Utilities|FlowControl|Delay 3.0)
      (CallFunction|CloseDoor))))

(event Custom|OpenDoor
  ;[1 1 1] Opens Door
  (Audio|PlaySound2D "/Game/sounds/q009/jumppad2.jumppad2" 1.0 1.0 0.0 0 0)
  (Components|MoveComponentTo (Variables|Default|GetDoor_Sprite) (Variables|/Script/Engine.SceneComponent|GetRelativeLocation (Variables|Default|GetDoorOpenLocation)) "0, 0, 0" true false 1.0 false))

(event Custom|CloseDoor
  ;[1 1 1] Close door
  (Audio|PlaySound2D "/Game/sounds/q009/jumppad2.jumppad2" 1.0 1.0 0.0 0 0)
  (Components|MoveComponentTo (Variables|Default|GetDoor_Sprite) (Variables|/Script/Engine.SceneComponent|GetRelativeLocation (Variables|Default|GetDoorStartLocation)) "0, 0, 0" false true 1.0 false))

(event EventBeginPlay)

(event Collision|EventActorBeginOverlap
  (params (OtherActor :type Actor%20Object%20Reference)))

(event EventTick
  (params (DeltaSeconds :type Float%20%28single-precision%29)))

(fn ConstructionScript)