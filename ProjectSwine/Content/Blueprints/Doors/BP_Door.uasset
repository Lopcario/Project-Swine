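; Key-card door that shows a colored sprite and removes itself once the player holds the matching key.
; BeginPlay uses KeyCardColor to set the orange or red sprite, leaving blue doors on their default sprite.
; Tick polls the matching key flag on BP_FirstPersonCharacter and destroys the door when it is true, with no overlap or proximity check.
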(event EventBeginPlay
  (if (not (== (Variables|Default|GetKeyCardColor) 1))
    (if (== (Variables|Default|GetKeyCardColor) 2)
      (Rendering|Components|Sprite|SetSprite (Variables|Default|Getdoor_Sprite) "/Game/Sprites/DevSpritesReplaceLater/RetroFPSAssets/Items/Orangedoor_Sprite.Orangedoor_Sprite")
      (elif (== (Variables|Default|GetKeyCardColor) 3)
        (Rendering|Components|Sprite|SetSprite (Variables|Default|Getdoor_Sprite) "/Game/Sprites/DevSpritesReplaceLater/RetroFPSAssets/Items/reddoor_Sprite.reddoor_Sprite")))))

(event Collision|EventActorBeginOverlap
  (params (OtherActor :type Actor%20Object%20Reference)))

(event EventTick
  (params (DeltaSeconds :type Float%20%28single-precision%29))
  (if (== (Variables|Default|GetKeyCardColor) 1)
    (bind _asbp_first_person_character (Utilities|Casting|CastToBP_FirstPersonCharacter (Game|GetPlayerCharacter 0)))
    (if (Variables|/Game/FirstPerson/Blueprints/BP_FirstPersonCharacter.BP_FirstPersonCharacter_C|GetHasBlueKey _asbp_first_person_character)
      (Actor|DestroyActor))
    (elif (== (Variables|Default|GetKeyCardColor) 2)
      (bind _asbp_first_person_character_2 (Utilities|Casting|CastToBP_FirstPersonCharacter (Game|GetPlayerCharacter 0)))
      (if (Variables|/Game/FirstPerson/Blueprints/BP_FirstPersonCharacter.BP_FirstPersonCharacter_C|GetHasOrangeKey _asbp_first_person_character_2)
        (Actor|DestroyActor))
      (elif (== (Variables|Default|GetKeyCardColor) 3)
        (bind _asbp_first_person_character_3 (Utilities|Casting|CastToBP_FirstPersonCharacter (Game|GetPlayerCharacter 0)))
        (if (Variables|/Game/FirstPerson/Blueprints/BP_FirstPersonCharacter.BP_FirstPersonCharacter_C|GetHasRedKey _asbp_first_person_character_3)
          (Actor|DestroyActor))))))

(fn ConstructionScript)