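; BP_KeyCard is a blue key card pickup that continually turns to face the first-person player.
; From BeginPlay it caches the player character and starts a self-recalling event with a tiny Delay, used in place of Tick, that interpolates its yaw toward the player.
; When that character type overlaps it, it calls BlueKeyObtained on the character and destroys itself.
; The FacePlayer function is an empty stub.
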(event Custom|facePLay
  (Transformation|SetActorRotation (Math|Rotator|MakeRotator 0.0 0.0 (.yaw (Math|Interpolation|RInterpTo (Transformation|GetActorRotation) (Math|Rotator|FindLookatRotation (Transformation|GetActorLocation) (Transformation|GetActorLocation (Variables|Default|GetAs%20BP%20First%20Person%20Character))) (Utilities|Time|GetWorldDeltaSeconds) 2e+01))))
  (Utilities|FlowControl|Delay 0.001)
  (CallFunction|FacePLay))

(event EventBeginPlay
  (Utilities|FlowControl|Sequence
    (:then_1
      (bind _asbp_first_person_character (Utilities|Casting|CastToBP_FirstPersonCharacter (Game|GetPlayerCharacter 0)))
      (Variables|Default|SetAs%20BP%20First%20Person%20Character _asbp_first_person_character)
      (CallFunction|FacePLay))))

(event Collision|EventActorBeginOverlap
  (params (OtherActor :type Actor%20Object%20Reference))
  (bind _asbp_first_person_character (Utilities|Casting|CastToBP_FirstPersonCharacter OtherActor))
  (Default|BlueKeyObtained _asbp_first_person_character)
  (Actor|DestroyActor))

(event EventTick
  (params (DeltaSeconds :type Float%20%28single-precision%29)))

(fn ConstructionScript)

(fn FacePlayer)