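; BP_PickupBullets is a multipurpose sprite pickup that grants small or large health, armor, bullets or shells to the first-person character.
; PickupMode selects the sprite at BeginPlay, with both health sizes sharing one sprite.
; A self-recalling FacePlayer event with a tiny Delay, used instead of Tick, smoothly yaws the actor toward the player.
; On overlap with BP_FirstPersonCharacter, it calls that mode's pickup function and destroys itself.
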(event Custom|Face%20Player
  ;[1 1 1] face player
  (Transformation|SetActorRotation (Math|Rotator|MakeRotator 0.0 0.0 (.yaw (Math|Interpolation|RInterpTo (Transformation|GetActorRotation) (Math|Rotator|FindLookatRotation (Transformation|GetActorLocation) (Transformation|GetActorLocation (Variables|Default|GetCharRef))) (Utilities|Time|GetWorldDeltaSeconds) 2e+01))))
  (Utilities|FlowControl|Delay 0.001)
  (CallFunction|FacePlayer))

(event EventBeginPlay
  (Utilities|FlowControl|Sequence
    (:then_0
      (if (== (Variables|Default|GetPickupMode) 0)
        (Rendering|Components|Sprite|SetSprite (Variables|Default|GetAmmo_Sprite) "/Game/Sprites/DevSprites(ReplaceLater)/RetroFPSAssets/Items/Health_Sprite.Health_Sprite" :!label _label)
        (elif (== (Variables|Default|GetPickupMode) 1)
          (goto _label)
          (elif (== (Variables|Default|GetPickupMode) 2)
            (Rendering|Components|Sprite|SetSprite (Variables|Default|GetAmmo_Sprite) "/Game/Sprites/DevSprites(ReplaceLater)/RetroFPSAssets/Items/Armor_Sprite.Armor_Sprite")
            (elif (== (Variables|Default|GetPickupMode) 3)
              (Rendering|Components|Sprite|SetSprite (Variables|Default|GetAmmo_Sprite) "/Game/Sprites/DevSprites(ReplaceLater)/RetroFPSAssets/Items/Ammo_Sprite.Ammo_Sprite")
              (elif (== (Variables|Default|GetPickupMode) 4)
                (Rendering|Components|Sprite|SetSprite (Variables|Default|GetAmmo_Sprite) "/Game/Sprites/DevSprites(ReplaceLater)/RetroFPSAssets/Items/Shotgun_Sprite.Shotgun_Sprite")))))))
    (:then_1
      (bind _asbp_first_person_character (Utilities|Casting|CastToBP_FirstPersonCharacter (Game|GetPlayerCharacter 0)))
      (Variables|Default|SetCharRef _asbp_first_person_character)
      (CallFunction|FacePlayer))))

(event Collision|EventActorBeginOverlap
  (params (OtherActor :type Actor%20Object%20Reference))
  (bind _asbp_first_person_character (Utilities|Casting|CastToBP_FirstPersonCharacter OtherActor))
  (if (== (Variables|Default|GetPickupMode) 0)
    (Default|HPPickupSmall _asbp_first_person_character)
    (Actor|DestroyActor)
    (elif (== (Variables|Default|GetPickupMode) 1)
      (Default|HPPickupLarge _asbp_first_person_character)
      (Actor|DestroyActor)
      (elif (== (Variables|Default|GetPickupMode) 2)
        (Default|ArmorPickup _asbp_first_person_character)
        (Actor|DestroyActor)
        (elif (== (Variables|Default|GetPickupMode) 3)
          (Default|BulletPickup _asbp_first_person_character)
          (Actor|DestroyActor)
          (elif (== (Variables|Default|GetPickupMode) 4)
            (Default|ShellsPickup _asbp_first_person_character)
            (Actor|DestroyActor)))))))

(event EventTick
  (params (DeltaSeconds :type Float%20%28single-precision%29)))

(fn ConstructionScript)