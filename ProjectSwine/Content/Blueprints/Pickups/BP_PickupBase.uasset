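; Base pickup actor for weapons, health, armor and ammo, shown as a sprite that turns toward the player.
; IsWeapon and PickupMode pick the sprite on BeginPlay and the character function called on overlap.
; On collection it plays a random sound through the PlayPickupSound macro and destroys itself.
; Billboarding interpolates yaw toward the player in a self-calling FacePlayer event with a tiny Delay, instead of using Tick.
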(event Custom|Face%20Player
  ;[1 1 1] face player
  (Transformation|SetActorRotation (Math|Rotator|MakeRotator 0.0 0.0 (.yaw (Math|Interpolation|RInterpTo (Transformation|GetActorRotation) (Math|Rotator|FindLookatRotation (Transformation|GetActorLocation) (Transformation|GetActorLocation (Variables|Default|GetCharRef))) (Utilities|Time|GetWorldDeltaSeconds) 2e+01))))
  (Utilities|FlowControl|Delay 0.001)
  (CallFunction|FacePlayer))

(event EventBeginPlay
  ;[1 1 1] Change what pickup
  (Utilities|FlowControl|Sequence
    (:then_0
      (if (Variables|Default|GetIsWeapon)
        (if (== (Variables|Default|GetPickupMode) 0)
          (Rendering|Components|Sprite|SetSprite (Variables|Default|GetSprite) "/Game/Sprites/DevSpritesReplaceLater/RetroFPSAssets/Weapons/Chainsaw/csawa0_Sprite.csawa0_Sprite")
          (elif (== (Variables|Default|GetPickupMode) 1)
            (Rendering|Components|Sprite|SetSprite (Variables|Default|GetSprite) "/Game/Sprites/DevSpritesReplaceLater/RetroFPSAssets/Weapons/Pistol/pistol1_Sprite.pistol1_Sprite")
            (elif (== (Variables|Default|GetPickupMode) 2)
              (Rendering|Components|Sprite|SetSprite (Variables|Default|GetSprite) "/Game/Sprites/DevSpritesReplaceLater/RetroFPSAssets/Weapons/Shotgun/sgn2a0_Sprite.sgn2a0_Sprite")
              (elif (== (Variables|Default|GetPickupMode) 3)
                (Rendering|Components|Sprite|SetSprite (Variables|Default|GetSprite) "/Game/Sprites/DevSpritesReplaceLater/RetroFPSAssets/Weapons/MiniGun/mguna0_Sprite.mguna0_Sprite")))))
        (elif (== (Variables|Default|GetPickupMode) 0)
          (Rendering|Components|Sprite|SetSprite (Variables|Default|GetSprite) "/Game/Sprites/DevSpritesReplaceLater/RetroFPSAssets/Items/Health_Sprite.Health_Sprite" :!label _label)
          (elif (== (Variables|Default|GetPickupMode) 1)
            (goto _label)
            (elif (== (Variables|Default|GetPickupMode) 2)
              (Rendering|Components|Sprite|SetSprite (Variables|Default|GetSprite) "/Game/Sprites/DevSpritesReplaceLater/RetroFPSAssets/Items/Armor_Sprite.Armor_Sprite")
              (elif (== (Variables|Default|GetPickupMode) 3)
                (Rendering|Components|Sprite|SetSprite (Variables|Default|GetSprite) "/Game/Sprites/DevSpritesReplaceLater/RetroFPSAssets/Items/Ammo_Sprite.Ammo_Sprite")
                (elif (== (Variables|Default|GetPickupMode) 4)
                  (Rendering|Components|Sprite|SetSprite (Variables|Default|GetSprite) "/Game/Sprites/DevSpritesReplaceLater/RetroFPSAssets/Items/Shotgun_Sprite.Shotgun_Sprite"))))))))
    (:then_1
      (bind _asbp_first_person_character (Utilities|Casting|CastToBP_FirstPersonCharacter (Game|GetPlayerCharacter 0)))
      (Variables|Default|SetCharRef _asbp_first_person_character)
      (CallFunction|FacePlayer))))

(event Collision|EventActorBeginOverlap
  (params (OtherActor :type Actor%20Object%20Reference))
  ;[1 1 1] applies pickup
  (bind _asbp_first_person_character (Utilities|Casting|CastToBP_FirstPersonCharacter OtherActor))
  (Variables|Default|SetFirstPersonCharacterRef _asbp_first_person_character)
  (if (Variables|Default|GetIsWeapon)
    (if (== (Variables|Default|GetPickupMode) 0)
      (Default|EquipSaw (Variables|Default|GetFirstPersonCharacterRef))
      (Utilities|PlayPickupSound
        (:out
          (Actor|DestroyActor)))
      (elif (== (Variables|Default|GetPickupMode) 1)
        (Default|EquipPistol (Variables|Default|GetFirstPersonCharacterRef))
        (Utilities|PlayPickupSound
          (:out
            (Actor|DestroyActor)))
        (elif (== (Variables|Default|GetPickupMode) 2)
          (Default|EquipShotgun (Variables|Default|GetFirstPersonCharacterRef))
          (Utilities|PlayPickupSound
            (:out
              (Actor|DestroyActor)))
          (elif (== (Variables|Default|GetPickupMode) 3)
            (Default|EquipChaingun (Variables|Default|GetFirstPersonCharacterRef))
            (Utilities|PlayPickupSound
              (:out
                (Actor|DestroyActor)))))))
    (elif (== (Variables|Default|GetPickupMode) 0)
      (Default|HPPickupSmall (Variables|Default|GetFirstPersonCharacterRef))
      (Utilities|PlayPickupSound
        (:out
          (Actor|DestroyActor)))
      (elif (== (Variables|Default|GetPickupMode) 1)
        (Default|HPPickupLarge (Variables|Default|GetFirstPersonCharacterRef))
        (Utilities|PlayPickupSound
          (:out
            (Actor|DestroyActor)))
        (elif (== (Variables|Default|GetPickupMode) 2)
          (Default|ArmorPickup (Variables|Default|GetFirstPersonCharacterRef))
          (Utilities|PlayPickupSound
            (:out
              (Actor|DestroyActor)))
          (elif (== (Variables|Default|GetPickupMode) 3)
            (Default|BulletPickup (Variables|Default|GetFirstPersonCharacterRef))
            (Utilities|PlayPickupSound
              (:out
                (Actor|DestroyActor)))
            (elif (== (Variables|Default|GetPickupMode) 4)
              (Default|ShellsPickup (Variables|Default|GetFirstPersonCharacterRef))
              (Utilities|PlayPickupSound
                (:out
                  (Actor|DestroyActor))))))))))

(event EventTick
  (params (DeltaSeconds :type Float%20%28single-precision%29)))

(fn ConstructionScript)

(fn NewFunction
  (Audio|PlaySoundatLocation (.OutItem (Utilities|Array|Random (Variables|Default|GetSound))) (Transformation|GetWorldLocation (Variables|Default|GetSphere)) "0, 0, 0" 1.0 1.0 0.0 0 0 0 0))