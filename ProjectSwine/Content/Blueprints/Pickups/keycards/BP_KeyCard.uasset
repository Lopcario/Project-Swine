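; BP_KeyCard is a colored keycard pickup that grants the first-person character the matching key on overlap.
; KeyCardColor picks the blue, orange or red sprite at BeginPlay and selects which key-obtained event to call on the character.
; A self-recalling short-delay loop, used instead of Tick, yaws the sprite actor toward the player.
; On pickup, it plays a random sound at the sphere's location and destroys itself.
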(event Custom|facePLay
  ;[1 1 1] has sprite face player
  (Transformation|SetActorRotation (Math|Rotator|MakeRotator 0.0 0.0 (.yaw (Math|Interpolation|RInterpTo (Transformation|GetActorRotation) (Math|Rotator|FindLookatRotation (Transformation|GetActorLocation) (Transformation|GetActorLocation (Variables|Default|GetAs%20BP%20First%20Person%20Character))) (Utilities|Time|GetWorldDeltaSeconds) 2e+01))))
  (Utilities|FlowControl|Delay 0.001)
  (CallFunction|FacePLay))

(event EventBeginPlay
  (Utilities|FlowControl|Sequence
    (:then_0
      (bind _asbp_first_person_character (Utilities|Casting|CastToBP_FirstPersonCharacter (Game|GetPlayerCharacter 0)))
      (Variables|Default|SetAs%20BP%20First%20Person%20Character _asbp_first_person_character)
      (CallFunction|FacePLay))
    (:then_1
      (if (== (Variables|Default|GetKeyCardColor) 1)
        (Rendering|Components|Sprite|SetSprite (Variables|Default|GetKey_Sprite) "/Game/Sprites/DevSpritesReplaceLater/RetroFPSAssets/Items/bluekey_Sprite.bluekey_Sprite")
        (elif (== (Variables|Default|GetKeyCardColor) 2)
          (Rendering|Components|Sprite|SetSprite (Variables|Default|GetKey_Sprite) "/Game/Sprites/DevSpritesReplaceLater/RetroFPSAssets/Items/orangekey_Sprite.orangekey_Sprite")
          (elif (== (Variables|Default|GetKeyCardColor) 3)
            (Rendering|Components|Sprite|SetSprite (Variables|Default|GetKey_Sprite) "/Game/Sprites/DevSpritesReplaceLater/RetroFPSAssets/Items/redkey_Sprite.redkey_Sprite")))))))

(event Collision|EventActorBeginOverlap
  (params (OtherActor :type Actor%20Object%20Reference))
  ;[1 1 1] Unlocks doors when picked up
  (Variables|Default|SetOther%20Actor OtherActor)
  (if (== (Variables|Default|GetKeyCardColor) 1)
    (bind _asbp_first_person_character (Utilities|Casting|CastToBP_FirstPersonCharacter (Variables|Default|GetOther%20Actor)))
    (Default|BlueKeyObtained _asbp_first_person_character)
    (Utilities|Pickupsound
      (:NewParam2
        (Actor|DestroyActor)))
    (elif (== (Variables|Default|GetKeyCardColor) 2)
      (bind _asbp_first_person_character_2 (Utilities|Casting|CastToBP_FirstPersonCharacter (Variables|Default|GetOther%20Actor)))
      (Default|OrangeKeyObtained _asbp_first_person_character_2)
      (Utilities|Pickupsound
        (:NewParam2
          (Actor|DestroyActor)))
      (elif (== (Variables|Default|GetKeyCardColor) 3)
        (bind _asbp_first_person_character_3 (Utilities|Casting|CastToBP_FirstPersonCharacter (Variables|Default|GetOther%20Actor)))
        (Default|RedKeyObtained _asbp_first_person_character_3)
        (Utilities|Pickupsound
          (:NewParam2
            (Actor|DestroyActor)))))))

(event EventTick
  (params (DeltaSeconds :type Float%20%28single-precision%29)))

(fn ConstructionScript)

(fn FacePlayer)